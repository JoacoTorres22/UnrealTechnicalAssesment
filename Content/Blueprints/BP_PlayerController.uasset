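; Player controller that creates and shows the game's menu widgets.
; On BeginPlay, the UnrealTechnical level shows the game menu, while other levels show the main menu, pre-create gameplay, game and game-over widgets, and pause.
; PauseGame and UnPauseGame only add or remove the gameplay widget, while GameOverEvent pauses and shows the game-over screen.
; A SoundOn rep-notify stops the player tank's engine sound.
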(event `self.ReceiveBeginPlay`
  (bind _gamemenu (`self.GameMenu`))
  (bind _returnvalue (`GameplayStatics.GetCurrentLevelName` true))
  (if (`KismetStringLibrary.EqualEqual_StrStr` _returnvalue "UnrealTechnical")
    (`/Engine/EditorBlueprintResources/StandardMacros.IsValid` _gamemenu
      (:`Is Valid`
        _)
      (:`Is Not Valid`
        (bind _returnvalue_2 (`|CreateWidget` "/Game/UMG/WBP_GameMenu.WBP_GameMenu_C" self))
        (bind _output_get (set `self.GameMenu` _returnvalue_2))))
    (`UserWidget.AddToViewport` _gamemenu 0)
    (`UserWidget.AddToViewport` _output_get 0)
    (else
      (`|ExecutionSequence`
        (:`then_0`
          (bind _returnvalue_3 (`|CreateWidget` "/Game/UMG/WBP_MainMenu.WBP_MainMenu_C" self))
          (bind _output_get_2 (set `self.MainMenu` _returnvalue_3))
          (`UserWidget.AddToViewport` _output_get_2 0))
        (:`then_1`
          (bind _returnvalue_4 (`|CreateWidget` "/Game/UMG/WBP_Gameplay.WBP_Gameplay_C" self))
          (set `self.GamePlayMenu` _returnvalue_4))
        (:`then_2`
          (bind _returnvalue_5 (`|CreateWidget` "/Game/UMG/WBP_GameMenu.WBP_GameMenu_C" self))
          (set `self.GameMenu` _returnvalue_5))
        (:`then_3`
          (bind _returnvalue_6 (`|CreateWidget` "/Game/UMG/WBP_GameOver.WBP_GameOver_C" self))
          (set `self.GameOver` _returnvalue_6))
        (:`then_4`
          (`GameplayStatics.SetGamePaused` true))))))

(event `self.ReceiveTick`
  (params (DeltaSeconds :type "Float (single-precision)")))

(fn `GameOverEvent`
  (bind _gameover (`self.GameOver`))
  (`GameplayStatics.SetGamePaused` true)
  (`/Engine/EditorBlueprintResources/StandardMacros.IsValid` _gameover
    (:`Is Valid`
      _)
    (:`Is Not Valid`
      (bind _returnvalue (`|CreateWidget` "/Game/UMG/WBP_GameOver.WBP_GameOver_C"))
      (bind _output_get (set `self.GameOver` _returnvalue))))
  (`UserWidget.AddToViewport` _gameover 0)
  (`UserWidget.AddToViewport` _output_get 0))

(fn `OnRep_SoundOn`
  (`AudioComponent.Stop` (`/Game/Blueprints/BP_Tank.EngineSound` (cast `/Game/Blueprints/BP_Tank` (`GameplayStatics.GetPlayerPawn` 0) :!pure true))))

(fn `PauseGame`
  (bind _gameplaymenu (`self.GamePlayMenu`))
  (`/Engine/EditorBlueprintResources/StandardMacros.IsValid` _gameplaymenu
    (:`Is Valid`
      _)
    (:`Is Not Valid`
      (bind _returnvalue (`|CreateWidget` "/Game/UMG/WBP_Gameplay.WBP_Gameplay_C" self))
      (bind _output_get (set `self.GamePlayMenu` _returnvalue))))
  (`UserWidget.AddToViewport` _gameplaymenu 0)
  (`UserWidget.AddToViewport` _output_get 0))

(fn `unPauseGame`
  (`Widget.RemoveFromParent` (`self.GamePlayMenu`)))

(fn `UserConstructionScript`)