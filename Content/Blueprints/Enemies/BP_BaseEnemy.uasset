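; Base enemy for a tank game that dies when its sphere is overlapped, scoring a point for the player's BP_Tank.
; BeginPlay loads saved high scores into the tank.
; Overlap destroys the other actor, plays a Niagara effect, then after a delay destroys itself and increments Points.
; Only when Points beats the lowest high score does it update and save the list, decrement GameInstance's enemy count and, at zero, trigger game over and EndMenu.
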(event `self.ReceiveBeginPlay`
  (set `self.Tank` (cast `/Game/Blueprints/BP_Tank` (`GameplayStatics.GetPlayerPawn` 0) :!pure true))
  (bind _returnvalue (`GameplayStatics.DoesSaveGameExist` (`self.SlotName`)))
  (if _returnvalue
    (bind _returnvalue_2 (`GameplayStatics.LoadGameFromSlot` (`self.SlotName`)))
    (bind _output_get (set `self.SaverSubClass` _returnvalue_2))
    (bind _asbp_save_highscore (cast `/Game/Blueprints/BP_SaveHighscore` _output_get))
    (set `/Game/Blueprints/BP_Tank.HighScore` (`/Game/Blueprints/BP_SaveHighscore.HighScore` _asbp_save_highscore) (`self.Tank`))))

(event `self.Sphere.OnComponentBeginOverlap`
  (params (OverlappedComponent :type "PrimitiveComponent Object Reference") (OtherActor :type "Actor Object Reference") (OtherComp :type "PrimitiveComponent Object Reference") (OtherBodyIndex :type Integer) (bFromSweep :type Boolean) (SweepResult :type "HitResult Structure (by ref)"))
  (bind _sphere (`self.Sphere`))
  (bind _asbp_tank (cast `/Game/Blueprints/BP_Tank` (`GameplayStatics.GetPlayerPawn` 0) :!pure true))
  (bind _highscore (`/Game/Blueprints/BP_Tank.HighScore` _asbp_tank))
  (bind (_indexofminvalue _minvalue) (`KismetMathLibrary.MinOfIntArray` _highscore))
  (`self.K2_DestroyActor` OtherActor)
  (`SceneComponent.SetVisibility` _sphere false false)
  (`AddComponent|NODE_AddNiagaraComponent-0` :`RelativeTransform` (`KismetMathLibrary.MakeTransform` (`SceneComponent.RelativeLocation` _sphere)))
  (`KismetSystemLibrary.Delay` 1.0)
  (`self.K2_DestroyActor`)
  (bind _result (`/Engine/EditorBlueprintResources/StandardMacros.IncrementInt` (`/Game/Blueprints/BP_Tank.Points` _asbp_tank))
    (:`  `
      (if (> _result _minvalue)
        (if (> (`KismetArrayLibrary.Array_Length` _highscore) 3)
          (`KismetArrayLibrary.Array_Remove` _highscore _indexofminvalue))
        (`KismetArrayLibrary.Array_Add` _highscore _result)
        (bind _returnvalue (`GameplayStatics.DoesSaveGameExist` (`self.SlotName`)))
        (if _returnvalue
          (bind _returnvalue_2 (`GameplayStatics.LoadGameFromSlot` (`self.SlotName`)))
          (bind _output_get (set `self.SaverSubClass` _returnvalue_2))
          (bind _asbp_save_highscore (cast `/Game/Blueprints/BP_SaveHighscore` _output_get))
          (set `/Game/Blueprints/BP_SaveHighscore.HighScore` _highscore _asbp_save_highscore)
          (`GameplayStatics.SaveGameToSlot` (`self.SaverSubClass`) (`self.SlotName`))
          (else
            (bind _returnvalue_3 (`GameplayStatics.CreateSaveGameObject` "/Game/Blueprints/BP_SaveHighscore.BP_SaveHighscore_C"))
            (bind _output_get_2 (set `self.SaverSubClass` _returnvalue_3))
            (bind _asbp_save_highscore_2 (cast `/Game/Blueprints/BP_SaveHighscore` _output_get_2))
            (set `/Game/Blueprints/BP_SaveHighscore.HighScore` _highscore _asbp_save_highscore_2)
            (`GameplayStatics.SaveGameToSlot` (`self.SaverSubClass`) (`self.SlotName`))))
        (`/Engine/EditorBlueprintResources/StandardMacros.DecrementInt` (`/Game/Blueprints/BP_GameInstance.NumberOfEnemies` (cast `/Game/Blueprints/BP_GameInstance` (`GameplayStatics.GetGameInstance`) :!pure true))
          (:`  `
            (if (<= (`/Game/Blueprints/BP_GameInstance.NumberOfEnemies` (cast `/Game/Blueprints/BP_GameInstance` (`GameplayStatics.GetGameInstance`) :!pure true)) 0)
              (`GameplayStatics.OpenLevel` "EndMenu")
              (`/Game/Blueprints/BP_PlayerController.GameOverEvent` (cast `/Game/Blueprints/BP_PlayerController` (`GameplayStatics.GetPlayerController` 0) :!pure true)))))))))

(fn `UserConstructionScript`)