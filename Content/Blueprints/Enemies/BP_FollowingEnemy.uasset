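; Enemy pawn that follows the player, caching the first player controller's pawn on BeginPlay.
; Every tick it yaws to face the player, updates its speed and reissues an AI MoveTo toward the player's location with a wide acceptance radius.
; Its FloatingPawnMovement max speed derives from the absolute difference between player distance and a small offset, clamped to a low cap.
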(event `self.ReceiveBeginPlay`
  (`parent.ReceiveBeginPlay`)
  (set `self.Player` (`Controller.K2_GetPawn` (`GameplayStatics.GetPlayerController` 0))))

(event `self.ReceiveTick`
  (params (DeltaSeconds :type "Float (single-precision)"))
  (`parent.ReceiveTick` DeltaSeconds)
  (`self.LookPlayer`)
  (`self.SetSpeed`)
  (`|AIMoveTo` self (`self.K2_GetActorLocation` (`self.Player`)) null 500.0))

(fn `LookPlayer`
  (bind (_returnvalue_roll _returnvalue_pitch _returnvalue_yaw) (`KismetMathLibrary.BreakRotator` (`KismetMathLibrary.FindLookAtRotation` (`self.K2_GetActorLocation`) (`self.K2_GetActorLocation` (`self.Player`)))))
  (`self.K2_SetActorRotation` (`KismetMathLibrary.MakeRotator` 0.0 0.0 _returnvalue_yaw)))

(fn `SetSpeed`
  (set `FloatingPawnMovement.MaxSpeed` (`KismetMathLibrary.FClamp` (`KismetMathLibrary.Abs` (- (`KismetMathLibrary.Vector_Distance` (`self.K2_GetActorLocation`) (`self.K2_GetActorLocation` (`self.Player`))) 35.0)) 0.0 50.0) (`self.FloatingPawnMovement`)))

(fn `UserConstructionScript`
  (`parent.UserConstructionScript`))