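; Player-controlled tank pawn that possesses itself with the first player controller on BeginPlay.
; Axis inputs drive it along the Core forward vector, yaw the root, and aim separately by yawing the turret and pitching the cannon pivot within clamped limits.
; Shot spawns a BP_Projectile at the bullet location, pushes it along the cannon's forward vector and plays an explosion sound.
; BlockMouse toggles cursor visibility and input mode.
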(event `self.ReceiveBeginPlay`
  (`Controller.Possess` (`GameplayStatics.GetPlayerController` 0) self))

(event `InputAxis|RotateTurret`
  (params (AxisValue :type "Float (single-precision)"))
  (`self.RotateTurret` AxisValue))

(event `InputAction|BlockMouse`
  (params (Key :type "Key Structure"))
  (bind _returnvalue (`GameplayStatics.GetPlayerController` 0))
  (bind _returnvalue_2 (`GameplayStatics.GetPlayerController` 0))
  (:`Pressed`
    (`/Engine/EditorBlueprintResources/StandardMacros.FlipFlop`
      (:`A`
        (`WidgetBlueprintLibrary.SetInputMode_GameOnly` _returnvalue)
        (set `PlayerController.bShowMouseCursor` false _returnvalue))
      (:`B`
        (`WidgetBlueprintLibrary.SetInputMode_GameAndUIEx` _returnvalue_2 null)
        (set `PlayerController.bShowMouseCursor` true _returnvalue_2)))))

(event `InputAxis|InclineTurret`
  (params (AxisValue :type "Float (single-precision)"))
  (`self.Incline Turret` AxisValue))

(event `InputAxis|MoveForward`
  (params (AxisValue :type "Float (single-precision)"))
  (`self.AddMovementInput` self (* (`SceneComponent.GetForwardVector` (`self.Core`)) (`self.Direction`)) (* AxisValue (`self.MovementSpeed`)) false))

(event `InputAxis|TurnRight`
  (params (AxisValue :type "Float (single-precision)"))
  (`SceneComponent.K2_AddWorldRotation` (`self.DefaultSceneRoot`) (`KismetMathLibrary.MakeRotator` 0.0 0.0 AxisValue) false false))

(event `InputAction|Shot`
  (params (Key :type "Key Structure"))
  (:`Pressed`
    (bind _returnvalue (`|SpawnActorFromClass` "/Game/Blueprints/BP_Projectile.BP_Projectile_C" (`KismetMathLibrary.MakeTransform` (`SceneComponent.K2_GetComponentLocation` (`self.BulletLocation`))) "AlwaysSpawn" "OverrideRootScale" null null))
    (`/Game/Blueprints/BP_Projectile.AddForce` _returnvalue (`SceneComponent.GetForwardVector` (`self.Cannon`)) (`self.ProjectileForce`))
    (`AudioComponent.Play` (`self.Explosion_2_-_SFX_Producer`) 0.0)))

(fn `Incline Turret`
  (params (Delta :type "Float (double-precision)"))
  (bind _cannoncenter (`self.CannonCenter`))
  (bind (_relativerotation_roll _relativerotation_pitch) (`KismetMathLibrary.BreakRotator` (`SceneComponent.RelativeRotation` _cannoncenter)))
  (if true
    (`SceneComponent.K2_AddRelativeRotation` _cannoncenter (`KismetMathLibrary.MakeRotator` 0.0 Delta) false false)
    (`SceneComponent.K2_SetRelativeRotation` _cannoncenter (`KismetMathLibrary.MakeRotator` 0.0 (`KismetMathLibrary.FClamp` _relativerotation_pitch (`self.MinInclination`) (`self.MaxInclination`))) false false)))

(fn `RotateTurret`
  (params (Delta :type "Float (double-precision)"))
  (`SceneComponent.K2_AddWorldRotation` (`self.Turret`) (`KismetMathLibrary.MakeRotator` 0.0 0.0 Delta) false false))

(fn `UserConstructionScript`)